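; Exposure component, apparently a base class, that tracks an entity's buildup of a given exposure type.
; AddCurrentExposure checks the exposure type, adds the amount scaled down by ExposureResistance, then fires the AddExposureValue dispatcher with that type, printing debug strings along the way.
; Getters return the single current value, and HasExposureVariant is a stub that always returns false.
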(event `/Game/BP/1_Entities/0_E_Components/Exposure/BPI_Expose.AddCurrentExposure`
  (params (ExposureType :type "/Game/BP/1_Entities/0_E_Components/Exposure/Enums/E_ExposureType Enum" :default "NewEnumerator0") (ExposureAmount :type "Float (double-precision)"))
  (`KismetSystemLibrary.PrintString` "Being Called")
  (if (`|EnumEquality` (`self.Exposure Type`) ExposureType)
    (set `self.CurrentExposure` (+ (`self.CurrentExposure`) (/ ExposureAmount (`self.ExposureResistance`))))
    (`self.AddExposureValue` ExposureType) ; Call Component Exposure, in player
    (`KismetSystemLibrary.PrintString` "Called Event Dispatcher, Add Exposure")))

(fn `GetCurrentExposure`
  (params (ExposureType :type "/Game/BP/1_Entities/0_E_Components/Exposure/Enums/E_ExposureType Enum" :default "NewEnumerator0"))
  (returns (`Current Exposure` :type "Float (double-precision)"))
  (return (`self.CurrentExposure`)))

(fn `HasExposureVariant`
  (params (SearchedExposureType :type "/Game/BP/1_Entities/0_E_Components/Exposure/Enums/E_ExposureType Enum" :default "NewEnumerator0"))
  (returns (HasSelectedExposure :type Boolean))
  (return false))

(fn `Return Current Exposure`
  (returns (CurrentExposure :type "Float (double-precision)"))
  (return (`self.CurrentExposure`)))