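; BP_C_E_Health is an entity health component that stores current health, maximum health and a regen amount.
; A getter returns all three stats, and separate setters update each, with only current health clamped between zero and the maximum.
; HealHealth adds the regen amount once per call through the clamped setter; the component's event graph has no active logic, so it does not trigger healing itself.
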(fn `Get Health Stats`
  (returns (CurrentHealth :type "Float (double-precision)") (MaxHealth :type "Float (double-precision)") (HealthRegen :type "Float (double-precision)"))
  (return (`self.CurrentHealth`) (`self.MaxHealth`) (`self.HealthRegen`)))

(fn `HealHealth`
  (bind (_currenthealth _maxhealth _healthregen) (`self.Get Health Stats`))
  (`self.Set Current Health` (+ _currenthealth _healthregen))
  (return))

(fn `Set Current Health`
  (params (CurrentHealth :type "Float (double-precision)"))
  (set `self.CurrentHealth` (`KismetMathLibrary.FClamp` CurrentHealth 0.0 (`.MaxHealth` (`self.Get Health Stats`))))
  (return))

(fn `Set HPRegen`
  (params (HealthRegen :type "Float (double-precision)"))
  (set `self.HealthRegen` HealthRegen)
  (return))

(fn `Set MaxHealth`
  (params (MaxHealth :type "Float (double-precision)"))
  (set `self.MaxHealth` MaxHealth)
  (return))