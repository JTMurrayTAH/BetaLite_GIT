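; BP_B_Entity is an entity actor Blueprint that exposes its exposure components through a common interface for adding and querying exposure by type.
; On BeginPlay it caches every BP_C_B_E_Exposure component in an array and prints their names.
; AddCurrentExposure forwards type and amount to every cached component without filtering.
; GetCurrentExposure and HasExposureVariant search the array by ExposureType to return a value or report a match.
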(event `self.ReceiveBeginPlay`
  (`self.SetUpExposureComponentArray`))

(event `/Game/BP/1_Entities/0_E_Components/Exposure/BPI_Expose.AddCurrentExposure`
  (params (ExposureType :type "/Game/BP/1_Entities/0_E_Components/Exposure/Enums/E_ExposureType Enum" :default "NewEnumerator0") (ExposureAmount :type "Float (double-precision)"))
  (`KismetSystemLibrary.PrintString` "Trying to Add Current Exposure")
  (for _array_element (`self.ExposureComponents`)
    (`/Game/BP/1_Entities/0_E_Components/Exposure/BPI_Expose.AddCurrentExposure` _array_element ExposureType ExposureAmount)))

(fn `GetCurrentExposure`
  (params (ExposureType :type "/Game/BP/1_Entities/0_E_Components/Exposure/Enums/E_ExposureType Enum" :default "NewEnumerator0"))
  (returns (`Current Exposure` :type "Float (double-precision)"))
  (for _array_element (`self.ExposureComponents`)
    (if (`|EnumEquality` (`/Game/BP/1_Entities/0_E_Components/Exposure/BP_C_B_E_Exposure.Exposure Type` _array_element) ExposureType)
      (break)))
  (return (`/Game/BP/1_Entities/0_E_Components/Exposure/BP_C_B_E_Exposure.CurrentExposure` _array_element)))

(fn `HasExposureVariant`
  (params (SearchedExposureType :type "/Game/BP/1_Entities/0_E_Components/Exposure/Enums/E_ExposureType Enum" :default "NewEnumerator0"))
  (returns (HasSelectedExposure :type Boolean))
  (for _array_element (`self.ExposureComponents`)
    (if (`|EnumEquality` SearchedExposureType (`/Game/BP/1_Entities/0_E_Components/Exposure/BP_C_B_E_Exposure.Exposure Type` _array_element))
      (return true))))

(fn `SetUpExposureComponentArray`
  (bind _output_get (set `self.ExposureComponents` (`self.K2_GetComponentsByClass` "/Game/BP/1_Entities/0_E_Components/Exposure/BP_C_B_E_Exposure.BP_C_B_E_Exposure_C")))
  (for _array_element _output_get
    (`KismetSystemLibrary.PrintString` (`KismetSystemLibrary.GetDisplayName` _array_element))))

(fn `UserConstructionScript`)