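; Hazard component for BP_Entity actors that tracks a hazard's type, amount, resistance and a keyed map of state values.
; Added hazard input is divided by resistance before accumulating, while state values can be set or incremented per key.
; Initialisation caches the owning BP_Entity and prints the component's name; despite its name, SetUpEventDelegates binds no events.
; GetOutData packs the current values into one output.
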(fn `Add Hazard State Value`
  (params (InputHazard :type "/Game/BP/Entites/0_Entity_Components/HazardComponents/Data/BP_E_HazardStrength Enum (by ref)") (InputValue :type "Float (double-precision) (by ref)"))
  (`BlueprintMapLibrary.Map_Add` (`self.HazardState`) (`local.InputHazard`) (+ (`BlueprintMapLibrary.Map_Find` (`self.HazardState`) (`local.InputHazard`)) (`local.InputValue`)))
  (return))

(fn `Add Hazard Value`
  (params (HazardInput :type "Float (double-precision)"))
  (set `self.HazardAmount` (+ (`self.HazardAmount`) (/ (`local.HazardInput`) (`self.HazardResistance`))))
  (return))

(fn `GetOutData`
  (returns (Output_Get :type "/Game/BP/Entites/0_Entity_Components/HazardComponents/BP_S_HazardData Structure"))
  (bind _output_get (set `self.HazardOutData` (make `/Game/BP/Entites/0_Entity_Components/HazardComponents/BP_S_HazardData` (`self.HazardType`) (`self.HazardAmount`) (`self.HazardResistance`) (`self.HazardState`))))
  (return _output_get))

(fn `InitaliseSelf`
  (`self.SetUpEventDelegates`)
  (`KismetSystemLibrary.PrintString` (`KismetSystemLibrary.GetDisplayName` self)))

(fn `SetHazardAmount`
  (params (HazardAmount :type "Float (double-precision)"))
  (set `self.HazardAmount` HazardAmount)
  (return))

(fn `SetHazardResistance`
  (params (HazardResistance :type "Float (double-precision)"))
  (set `self.HazardResistance` HazardResistance)
  (return))

(fn `SetHazardStateValue`
  (params (Key :type "/Game/BP/Entites/0_Entity_Components/HazardComponents/Data/BP_E_HazardStrength Enum (by ref)") (Value :type "Float (double-precision) (by ref)"))
  (`BlueprintMapLibrary.Map_Add` (`self.HazardState`) Key Value)
  (return))

(fn `SetUpEventDelegates`
  (bind _asbp_entity (cast `/Game/BP/Entites/BP_Entity` (`self.GetOwner`)))
  (set `self.HazardOwner` _asbp_entity)
  (return))