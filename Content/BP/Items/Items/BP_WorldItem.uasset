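; World item actor that shows the static mesh defined by its assigned item data class.
; The construction script runs Config, which instantiates that class as a data object, rebuilding it if the class differs, then updates the mesh.
; An unloaded soft mesh reference triggers an async load, whose immediate Then output, rather than a completion pin, re-runs the mesh update.
; SetItemData only stores the class, without refreshing object or mesh.
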(event `LoadItemMesh`
  (params (`Soft Ref` :type "StaticMesh Soft Object Reference"))
  (if (`KismetSystemLibrary.IsValidSoftObjectReference` `Soft Ref`)
    (`|LoadAsset` `Soft Ref`
      (:`then`
        (`self.Update Item Mesh`)))))

(fn `Config`
  (`self.ItemData`
    (:`then`
      (`self.ItemData_Obj`
        (:`then`
          (`self.IsObjSameAsClass`))
        (:`else`
          (`self.Construct Item Data Obj`)))
      (`self.Update Item Mesh`))
    (:`else`
      (return))))

(fn `Construct Item Data Obj`
  (bind _itemdata (`self.GetItemData`))
  (if (`KismetSystemLibrary.IsValidClass` _itemdata)
    (bind _returnvalue (`|GenericCreateObject` _itemdata))
    (set `self.ItemData_Obj` _returnvalue)
    (return)
    (else
      (`|VariableSetRef` (`self.ItemData_Obj`))
      (return))))

(fn `GetItemData`
  (returns (ItemData :type "/Game/BP/Items/Data/BP_ItemData Class Reference"))
  (return (`self.ItemData`)))

(fn `IsObjSameAsClass`
  (if (== (`GameplayStatics.GetObjectClass` (`self.ItemData_Obj`)) (`self.ItemData`))
    (return)
    (else
      (`self.Construct Item Data Obj`)
      (return))))

(fn `SetItemData`
  (params (ItemDataInput :type "/Game/BP/Items/Data/BP_ItemData Class Reference"))
  (set `self.ItemData` ItemDataInput)
  (return))

(fn `Update Item Mesh`
  (bind _itemdata_obj (`self.ItemData_Obj`)
    (:`then`
      (bind _mesh (`/Game/BP/Items/Data/BP_ItemData.Mesh` _itemdata_obj))
      (bind _output (`|ConvertAsset` _mesh))
      (`/Engine/EditorBlueprintResources/StandardMacros.IsValid` _output
        (:`Is Valid`
          (`StaticMeshComponent.SetStaticMesh` (`self.ItemMesh`) _output))
        (:`Is Not Valid`
          (`self.LoadItemMesh` _mesh))))
    (:`else`
      (`StaticMeshComponent.SetStaticMesh` (`self.ItemMesh`) null)
      (return))))

(fn `UserConstructionScript`
  (`self.Config`))